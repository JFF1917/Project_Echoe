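; BP_Leaf is a Paper2D leaf actor whose flipbook turns in quarter-turn steps each time its Rotate event is called.
; A timeline track named 120BPM drives a yaw lerp from the current rotation to 90 degrees further, suggesting beat-matched timing.
; When IsEnd is set, the finished timeline clears the flipbook and restores the rotation captured in the construction script.
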(event `Rotate`
  (params (`IsEnd?` :type Boolean))
  (bind (_rotation_roll _rotation_pitch _rotation_yaw) (`KismetMathLibrary.BreakRotator` (`self.Rotation`)))
  (set `self.Rotation` (`SceneComponent.K2_GetComponentRotation` (`self.PaperFlipbook`)))
  (bind (_direction _120bpm) (`Timeline|时间轴` :!via `PlayFromStart`)
    (:`Update`
      (`SceneComponent.K2_SetWorldRotation` (`self.PaperFlipbook`) (`KismetMathLibrary.MakeRotator` _rotation_roll _rotation_pitch (`KismetMathLibrary.Lerp` _rotation_yaw (+ _rotation_yaw 90.0) _120bpm)) false false))
    (:`Finished`
      (if `IsEnd?`
        (`PaperFlipbookComponent.SetFlipbook` (`self.PaperFlipbook`) null)
        (`SceneComponent.K2_SetWorldRotation` (`self.PaperFlipbook`) (`self.InitialRotation`) false false)))))

(fn `UserConstructionScript`
  (set `self.InitialRotation` (`SceneComponent.K2_GetComponentRotation` (`self.PaperFlipbook`))))