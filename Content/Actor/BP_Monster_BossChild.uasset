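; BP_Monster_BossChild is a Paper2D monster Blueprint, apparently a boss minion, that customizes what happens when it dies.
; Its MonsterDie event prints a "BOSS HP-1" debug message, clears WillPlayerMove, hides the flipbook and disables AOE and self collision, without destroying the actor.
; No boss health is changed here; BeginPlay is disabled and construction only calls the parent.
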(event `self.MonsterDie`
  ;[1 1 1] 注释
  (`KismetSystemLibrary.PrintString` "BOSS HP-1" true true (struct :`R` 0.807249 :`B` 1.0 :`A` 1.0) 5.0)
  (set `self.WillPlayerMove?` false)
  (`SceneComponent.SetVisibility` (`self.PaperFlipbook`) false false)
  (`PrimitiveComponent.SetCollisionEnabled` (`self.AoeCollision`) "NoCollision")
  (`PrimitiveComponent.SetCollisionEnabled` (`self.SelfCollission`) "NoCollision"))

(fn `UserConstructionScript`
  (`parent.UserConstructionScript`))