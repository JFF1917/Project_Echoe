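; Beat-driven boss monster that alternates at random between two multi-phase attacks, with a wait between them.
; MonsterAction runs a state machine in four-beat steps.
; Skill A reveals a random sword group in a red/blue pattern with shields, fires it, then toggles ChildGroupA's AoE hazards.
; Skill B spawns BossChild_B cross and non-cross attackers at preset points, triggers their skill stages on set beats, then destroys them.
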(event `self.MonsterAction`
  (switch `string` (`self.State`)
    (:`Idle`
      (switch `int` (`self.Beat`)
        (:`0`
          (`self.SetBeat` :!label _label))
        (:`1`
          (goto _label))
        (:`2`
          (goto _label))
        (:`3`
          (`self.SetBeat`)
          ;[1 1 1] 注释
          (set `self.State` "SkillASpawnP1")
          (set `self.CurrentGroupNum` (`KismetMathLibrary.RandomInteger` 4))
          (set `self.SwordColorPattern` (select `int` (`KismetMathLibrary.RandomInteger` 2) :`0` (`self.SwordColorPatternA`) :`1` (`self.SwordColorPatternB`)))
          (set `self.Beat` 0))))
    (:`SkillASpawnP1`
      (switch `int` (`self.CurrentGroupNum`)
        (:`0`
          (`self.SkillAGroup_P1` (`self.SwordGroup1`) (`self.SwordColorPattern`)))
        (:`1`
          (`self.SkillAGroup_P1` (`self.SwordGroup2`) (`self.SwordColorPattern`)))
        (:`2`
          (`self.SkillAGroup_P1` (`self.SwordGroup3`) (`self.SwordColorPattern`)))
        (:`3`
          (`self.SkillAGroup_P1` (`self.SwordGroup4`) (`self.SwordColorPattern`)))))
    (:`SkillASpawnP2`
      (switch `int` (`self.CurrentGroupNum`)
        (:`0`
          (`self.SkillAGroup_P2` (`self.SwordGroup1`) (`self.SwordColorPattern`)))
        (:`1`
          (`self.SkillAGroup_P2` (`self.SwordGroup2`) (`self.SwordColorPattern`)))
        (:`2`
          (`self.SkillAGroup_P2` (`self.SwordGroup3`) (`self.SwordColorPattern`)))
        (:`3`
          (`self.SkillAGroup_P2` (`self.SwordGroup4`) (`self.SwordColorPattern`)))))
    (:`SkillACheckP1`
      (`self.Wait4Beats` "SkillACheckP2"))
    (:`SkillACheckP2`
      (switch `int` (`self.Beat`)
        (:`0`
          (`self.SetBeat` :!label _label_2))
        (:`1`
          (for _array_element (`self.CurrentGroup`)
            (`self.MonsterCharge` _array_element))
          (goto _label_2))
        (:`2`
          (goto _label_2))
        (:`3`
          (for _array_element_2 (`self.CurrentGroup`)
            (`SceneComponent.SetVisibility` (`/Game/Actor/BP_MonsterBase.PaperFlipbook` _array_element_2) false true)
            (`self.MonsterSkill` _array_element_2 0)
            (`/Game/Actor/BP_Monster_Sword.HideShield` _array_element_2))
          (`self.SetBeat`)
          (set `self.State` "ChildASpawnP1"))))
    (:`ChildASpawnP1`
      (switch `int` (`self.Beat`)
        (:`0`
          (`self.SetBeat` :!label _label_3))
        (:`1`
          (for _array_element_3 (`self.ChildGroupA`)
            (`self.MonsterCharge` _array_element_3))
          (goto _label_3))
        (:`2`
          (goto _label_3))
        (:`3`
          (for _array_element_4 (`self.ChildGroupA`)
            (`SceneComponent.SetVisibility` (`/Game/Actor/BP_MonsterBase.PaperFlipbook` _array_element_4) true false)
            (`PrimitiveComponent.SetCollisionEnabled` (`/Game/Actor/BP_MonsterBase.AoeCollision` _array_element_4) "QueryOnly")
            (`PrimitiveComponent.SetCollisionEnabled` (`/Game/Actor/BP_MonsterBase.SelfCollission` _array_element_4) "QueryOnly")
            (`self.MonsterSkill` _array_element_4 0))
          (`self.SetBeat`)
          (set `self.State` "ChildASpawnP2"))))
    (:`ChildASpawnP2`
      (`self.Wait4Beats` "ChildASpawnP3"))
    (:`ChildASpawnP3`
      (switch `int` (`self.Beat`)
        (:`0`
          (`self.SetBeat` :!label _label_4))
        (:`1`
          (goto _label_4))
        (:`2`
          (goto _label_4))
        (:`3`
          (for _array_element_5 (`self.ChildGroupA`)
            (`SceneComponent.SetVisibility` (`/Game/Actor/BP_MonsterBase.PaperFlipbook` _array_element_5) false false)
            (`PrimitiveComponent.SetCollisionEnabled` (`/Game/Actor/BP_MonsterBase.AoeCollision` _array_element_5) "NoCollision")
            (`PrimitiveComponent.SetCollisionEnabled` (`/Game/Actor/BP_MonsterBase.SelfCollission` _array_element_5) "NoCollision"))
          (`self.SetBeat`)
          (set `self.State` "Wait")
          (set `self.CurrentGroupNum` (`KismetMathLibrary.RandomInteger` 4))
          (set `self.SwordColorPattern` (select `int` (`KismetMathLibrary.RandomInteger` 2) :`0` (`self.SwordColorPatternA`) :`1` (`self.SwordColorPatternB`)))
          (set `self.Beat` 0))))
    (:`SkillBSpawnP1`
      (switch `int` (`self.Beat`)
        (:`0`
          (`self.SetBeat` :!label _label_5))
        (:`1`
          (`self.SpawnChildB` (`KismetMathLibrary.RandomIntegerInRange` 2 3) true)
          (goto _label_5))
        (:`2`
          (goto _label_5))
        (:`3`
          (bind _output_get (set `self.CurrentFirstAoeRingIndex` (`KismetMathLibrary.RandomInteger` 2)))
          (`self.SpawnChildB` _output_get)
          (`self.SetBeat`)
          (set `self.State` "SkillBSpawnP2"))))
    (:`SkillBSpawnP2`
      (switch `int` (`self.Beat`)
        (:`0`
          (`self.SetBeat` :!label _label_6))
        (:`1`
          (if (== (`self.CurrentFirstAoeRingIndex`) 0)
            (`self.SpawnChildB` 1)
            (goto _label_6)
            (else
              (`self.SpawnChildB` 0)
              (goto _label_6))))
        (:`2`
          (goto _label_6))
        (:`3`
          (`self.SetBeat`)
          (set `self.State` "SkillBCheckP1"))))
    (:`SkillBCheckP1`
      (switch `int` (`self.Beat`)
        (:`0`
          (`self.SetBeat` :!label _label_7))
        (:`1`
          (for _array_element_6 (`self.CurrentChildGroupB`)
            (`/Engine/EditorBlueprintResources/StandardMacros.IsValid` _array_element_6
              (:`Is Valid`
                (`self.MonsterSkill` _array_element_6 0))))
          (goto _label_7))
        (:`2`
          (goto _label_7))
        (:`3`
          (for _array_element_7 (`self.CurrentChildGroupB`)
            (`/Engine/EditorBlueprintResources/StandardMacros.IsValid` _array_element_7
              (:`Is Valid`
                (`self.MonsterSkill` _array_element_7 1))))
          (`self.SetBeat`)
          (set `self.State` "SkillBCheckP2"))))
    (:`SkillBCheckP2`
      (switch `int` (`self.Beat`)
        (:`0`
          (`self.SetBeat` :!label _label_8))
        (:`1`
          (for _array_element_8 (`self.CurrentChildGroupB`)
            (`/Engine/EditorBlueprintResources/StandardMacros.IsValid` _array_element_8
              (:`Is Valid`
                (`self.MonsterSkill` _array_element_8 2))))
          (goto _label_8))
        (:`2`
          (goto _label_8))
        (:`3`
          (for _array_element_9 (`self.CurrentChildGroupB`)
            (`/Engine/EditorBlueprintResources/StandardMacros.IsValid` _array_element_9
              (:`Is Valid`
                (`self.MonsterSkill` _array_element_9 3))))
          (`self.SetBeat`)
          (set `self.State` "SkillBCheckP3"))))
    (:`SkillBCheckP3`
      (switch `int` (`self.Beat`)
        (:`0`
          (`self.SetBeat` :!label _label_9))
        (:`1`
          (goto _label_9))
        (:`2`
          (goto _label_9))
        (:`3`
          (for _array_element_10 (`self.CurrentChildGroupB`)
            (`/Engine/EditorBlueprintResources/StandardMacros.IsValid` _array_element_10
              (:`Is Valid`
                (`self.K2_DestroyActor` _array_element_10))))
          (`self.SetBeat`)
          (set `self.State` "Wait")
          (`KismetArrayLibrary.Array_Clear` (`self.CurrentChildGroupB`)))))
    (:`Wait`
      (`self.Wait4Beats` (`KismetMathLibrary.SelectString` "SkillASpawnP1" "SkillBSpawnP1" (`KismetMathLibrary.RandomBool`))))))

(fn `SetSwordVisibility`
  (params (Group :type "Array of /Game/Actor/BP_Monster_Sword Object Reference") (GroupIndex :type Integer) (Visible :type Boolean) (`IsRed?` :type Boolean))
  (bind _output (`|GetArrayItem` Group GroupIndex))
  (bind _paperflipbook (`/Game/Actor/BP_MonsterBase.PaperFlipbook` _output))
  (`SceneComponent.SetVisibility` _paperflipbook Visible false)
  (bind _output_get (set `/Game/Actor/BP_Monster_Sword.IsRed?` `IsRed?` _output))
  (if _output_get
    (`PaperFlipbookComponent.SetFlipbook` _paperflipbook "/Game/Actor/Animation/Anim_Sword_Red.Anim_Sword_Red")
    (else
      (`PaperFlipbookComponent.SetFlipbook` _paperflipbook "/Game/Actor/Animation/Anim_Sword_Blue.Anim_Sword_Blue")))
  (`/Game/Actor/BP_Monster_Sword.ShowShield` _output)
  (return))

(fn `SkillAGroup_P1`
  (params (Group :type "Array of /Game/Actor/BP_Monster_Sword Object Reference (by ref)") (SwordColorPattern :type "Array of Boolean"))
  (bind _output (`|GetArrayItem` SwordColorPattern 1))
  (bind _output_get (set `self.CurrentGroup` Group))
  (switch `int` (`self.Beat`)
    (:`0`
      (`self.SetBeat` :!label _label))
    (:`1`
      (`self.SetSwordVisibility` _output_get 0 true (`|GetArrayItem` SwordColorPattern))
      (goto _label))
    (:`2`
      (goto _label))
    (:`3`
      (`self.SetSwordVisibility` _output_get 1 true _output)
      (`self.SetSwordVisibility` _output_get 2 true _output)
      (`self.SetBeat`)
      (set `self.State` "SkillASpawnP2")))
  (return))

(fn `SkillAGroup_P2`
  (params (Group :type "Array of /Game/Actor/BP_Monster_Sword Object Reference (by ref)") (SwordColorPattern :type "Array of Boolean"))
  (bind _output (`|GetArrayItem` SwordColorPattern 3))
  (bind _output_2 (`|GetArrayItem` SwordColorPattern 2))
  (bind _output_get (set `self.CurrentGroup` Group))
  (switch `int` (`self.Beat`)
    (:`0`
      (`self.SetBeat` :!label _label))
    (:`1`
      (`self.SetSwordVisibility` _output_get 3 true _output_2)
      (`self.SetSwordVisibility` _output_get 4 true _output_2)
      (goto _label))
    (:`2`
      (goto _label))
    (:`3`
      (`self.SetSwordVisibility` _output_get 5 true _output)
      (`self.SetSwordVisibility` _output_get 6 true _output)
      (`self.SetBeat`)
      (set `self.State` "SkillACheckP1")))
  (return))

(fn `SpawnChildB`
  (params (Index :type Integer) (`IsCross?` :type Boolean))
  (bind _returnvalue (`|SpawnActorFromClass` "/Game/Actor/BP_Monster_BossChild_B.BP_Monster_BossChild_B_C" (`KismetMathLibrary.MakeTransform` (`self.K2_GetActorLocation` (`|GetArrayItem` (`self.ChildGroupB1`) Index))) "Undefined" "MultiplyWithRoot" null `IsCross?` null))
  (`self.MonsterCharge` _returnvalue)
  (`KismetArrayLibrary.Array_Add` (`self.CurrentChildGroupB`) _returnvalue)
  (return))

(fn `UserConstructionScript`
  (`parent.UserConstructionScript`))

(fn `Wait4Beats`
  (params (NextState :type String))
  (switch `int` (`self.Beat`)
    (:`0`
      _)
    (:`1`
      _)
    (:`2`
      _)
    (:`3`
      (`self.SetBeat`)
      (set `self.State` NextState)
      (return)))
  (`self.SetBeat`))