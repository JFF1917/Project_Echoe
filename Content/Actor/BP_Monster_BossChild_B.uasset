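; Boss child monster variant whose area-of-effect skill uses either a cross or ring pattern, chosen by IsCross.
; The construction script sets the preview flipbook; MonsterSkill hides it and plays the effect animation matching Sort.
; In parallel, one collision box is resized through that pattern's extent array, with each check overwriting WillHitPlayer, so the last result counts.
; A hit alters player HP through the game mode.
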(event `SetAoeVFX`
  (params (Sort :type Integer))
  (if (`self.IsCross?`)
    (switch `int` Sort
      (:`0`
        (`PaperFlipbookComponent.SetFlipbook` (`self.AoeVFX`) "/Game/Actor/Animation/Anim_AoeX_0.Anim_AoeX_0"))
      (:`1`
        (`PaperFlipbookComponent.SetFlipbook` (`self.AoeVFX`) "/Game/Actor/Animation/Anim_AoeX_1.Anim_AoeX_1"))
      (:`2`
        (`PaperFlipbookComponent.SetFlipbook` (`self.AoeVFX`) "/Game/Actor/Animation/Anim_AoeX_2.Anim_AoeX_2"))
      (:`3`
        (`PaperFlipbookComponent.SetFlipbook` (`self.AoeVFX`) "/Game/Actor/Animation/Anim_AoeX_3.Anim_AoeX_3")))
    (else
      (switch `int` Sort
        (:`0`
          (`PaperFlipbookComponent.SetFlipbook` (`self.AoeVFX`) "/Game/Actor/Animation/Anim_AoeRing_0.Anim_AoeRing_0"))
        (:`1`
          (`PaperFlipbookComponent.SetFlipbook` (`self.AoeVFX`) "/Game/Actor/Animation/Anim_AoeRing_1.Anim_AoeRing_1"))
        (:`2`
          (`PaperFlipbookComponent.SetFlipbook` (`self.AoeVFX`) "/Game/Actor/Animation/Anim_AoeRing_2.Anim_AoeRing_2"))
        (:`3`
          (`PaperFlipbookComponent.SetFlipbook` (`self.AoeVFX`) "/Game/Actor/Animation/Anim_AoeRing_3.Anim_AoeRing_3"))))))

(event `self.MonsterSkill`
  (params (Sort :type Integer))
  (bind _aoevfx (`self.AoeVFX`))
  (`|ExecutionSequence`
    (:`then_0`
      ;[0 0 0] ChangeOnBeat
      (`self.SetAoeVFX` Sort)
      (`SceneComponent.SetVisibility` (`self.AoeVisual`) false false)
      (`SceneComponent.SetVisibility` _aoevfx true false)
      (`PaperFlipbookComponent.PlayFromStart` _aoevfx)
      (`KismetSystemLibrary.Delay` (`PaperFlipbookComponent.GetFlipbookLength` (`self.AoeVFX`)))
      (`SceneComponent.SetVisibility` (`self.AoeVFX`) false false))
    (:`then_1`
      (if (`self.IsCross?`)
        (switch `int` Sort
          (:`0`
            (`self.CheckAllAoeHit` (`self.AoeCrossBoxExtent0`)))
          (:`1`
            (`self.CheckAllAoeHit` (`self.AoeCrossBoxExtent1`)))
          (:`2`
            (`self.CheckAllAoeHit` (`self.AoeCrossBoxExtent2`)))
          (:`3`
            (`self.CheckAllAoeHit` (`self.AoeCrossBoxExtent3`))))
        (else
          (switch `int` Sort
            (:`0`
              (`self.CheckAllAoeHit` (`self.AoeRingBoxExtent0`)))
            (:`1`
              (`self.CheckAllAoeHit` (`self.AoeRingBoxExtent1`)))
            (:`2`
              (`self.CheckAllAoeHit` (`self.AoeRingBoxExtent2`)))
            (:`3`
              (`self.CheckAllAoeHit` (`self.AoeRingBoxExtent3`))))))
      (if (`self.Will Hit Player?`)
        (bind _asbp_my_game_mode (cast `/Game/Character/BP_MyGameMode` (`GameplayStatics.GetGameMode`)))
        (`/Game/Character/BP_MyGameMode.AlterPlayerHP` _asbp_my_game_mode "Skill" 1)
        (set `self.Will Hit Player?` false)
        (set `self.WillPlayerMove?` false)
        ;[1 1 1] 注释
        (`KismetSystemLibrary.PrintString` "被打了！！" true true (struct :`R` 1.0 :`G` 0.011477 :`A` 1.0) 10.0)))))

(fn `CheckAllAoeHit`
  (params (Array :type "Array of Vector Structure"))
  (for _array_element Array
    (`BoxComponent.SetBoxExtent` (`self.AoeCollision`) _array_element true)
    (bind _willhitplayer_ (`self.CheckSkillHit`))
    (set `self.Will Hit Player?` _willhitplayer_))
  (return))

(fn `UserConstructionScript`
  (`parent.UserConstructionScript`)
  (if (`self.IsCross?`)
    (`PaperFlipbookComponent.SetFlipbook` (`self.AoeVisual`) "/Game/Actor/Animation/Anim_AOECross.Anim_AOECross")
    (else
      (`PaperFlipbookComponent.SetFlipbook` (`self.AoeVisual`) "/Game/Actor/Animation/Anim_AoeRing.Anim_AoeRing"))))