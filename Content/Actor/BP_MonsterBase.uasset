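; Base monster for a beat-based, tile-stepping game, with placeholder patrol and active actions that specific monsters can fill in.
; MonsterAction dispatches over a four-beat cycle, then checks a discovery sphere that activates the monster with an aggro sound.
; Chase helpers turn along the dominant axis toward the player, then step by timeline or telegraph an AoE attack.
; Blocking and hit checks use the player's pending next step when moving, and hits damage through the GameMode.
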(event `self.ReceiveBeginPlay`
  (set `self.MonsterHP` (`self.MonsterHPMax`))
  (bind _asbp_player (cast `/Game/Character/BP_Player` (`GameplayStatics.GetPlayerCharacter` 0)))
  (set `self.ThePlayer` _asbp_player))

(event `CheckDiscovery`
  (if (`PrimitiveComponent.IsOverlappingComponent` (`self.DiscoverySphere`) (`Character.CapsuleComponent` (`self.ThePlayer`)))
    (`|ExecutionSequence`
      (:`then_0`
        (if (not (`self.IsActive?`))
          (`GameplayStatics.PlaySound2D` "/Game/SFX/FFXIV/FFXIV_Aggro.FFXIV_Aggro" 1.0 1.0 0.0 null null)))
      (:`then_1`
        (set `self.IsActive?` true)
        (`SceneComponent.SetVisibility` (`self.Discover`) true true)))))

(event `ActionCA1`
  (set `self.WillPlayerMove?` false :!label _label))

(event `ActionCA3`
  (goto _label))

(event `ActionCA2`
  (goto _label))

(event `ActionCA4`
  (goto _label))

(event `MonsterAction`
  (if (`self.IsActive?`)
    ;[0 0 0] DependOnSpecificMonster
    ;;[0 0 0] Chase&Attack
    (switch `int` (`self.Beat`)
      (:`0`
        (`self.ActionCA1`))
      (:`1`
        (`self.ActionCA2`))
      (:`2`
        (`self.ActionCA3`))
      (:`3`
        (`self.ActionCA4`)))
    (else
      ;;[0 0 0] Patrol
      (switch `int` (`self.Beat`)
        (:`0`
          (`self.ActionP1`))
        (:`1`
          (`self.ActionP2`))
        (:`2`
          (`self.ActionP3`))
        (:`3`
          (`self.ActionP4`)))))
  ;[1 1 1] 注释
  (`self.SetBeat`)
  (`Timeline|时间轴_0` :!via `PlayFromStart`
    (:`Finished`
      (`self.CheckDiscovery`))))

(event `ActionP1`
  (set `self.WillPlayerMove?` false :!label _label_2))

(event `ActionP3`
  (goto _label_2))

(event `ActionP2`
  (goto _label_2))

(event `ActionP4`
  (goto _label_2))

(event `MonsterActionVisual`)

(event `MonsterChasePlayer`
  (bind (_returnvalue_x _returnvalue_y) (`KismetMathLibrary.BreakVector` (- (`self.PlayerLocation`) (`self.MonsterLocation`))))
  (set `self.PlayerLocation` (`self.K2_GetActorLocation` (`self.ThePlayer`)))
  (set `self.MonsterLocation` (`self.K2_GetActorLocation`))
  (set `self.XDistance` _returnvalue_x)
  (set `self.YDIstance` _returnvalue_y)
  (if (>= (`KismetMathLibrary.Abs` (`self.XDistance`)) (`KismetMathLibrary.Abs` (`self.YDIstance`)))
    (if (> (`self.XDistance`) 10.0)
      (`self.MonsterTurnUp`)
      (if (`PrimitiveComponent.IsOverlappingComponent` (`self.AoeCollision`) (`Character.CapsuleComponent` (`self.ThePlayer`))) :!label _label_3
        (`self.MonsterAttack`)
        (elif (`self.WillPlayerMove?`)
          (if (`PrimitiveComponent.IsOverlappingComponent` (`self.NextStep`) (`/Game/Character/BP_Player.NextStep` (`self.ThePlayer`)))
            ;[1 1 1] 注释
            (`KismetSystemLibrary.PrintString` "被堵了" true true (struct :`R` 1.0 :`G` 0.08839 :`A` 1.0) 5.0)
            (else
              (`self.MonsterMove` :!label _label_4)))
          (elif (`PrimitiveComponent.IsOverlappingComponent` (`self.NextStep`) (`Character.CapsuleComponent` (`self.ThePlayer`)))
            _
            (else
              (goto _label_4)))))
      (set `self.WillPlayerMove?` false)
      (elif (< (`self.XDistance`) -10.0)
        (`self.MonsterTurnDown`)
        (goto _label_3)
        (else
          (`KismetSystemLibrary.PrintString` "追逐出错啦！！！" true true (struct :`R` 1.0 :`G` 0.08839 :`A` 1.0) 5.0 :!label _label_5))))
    (elif (> (`self.YDIstance`) 10.0)
      (`self.MonsterTurnRight`)
      (goto _label_3)
      (elif (< (`self.YDIstance`) -10.0)
        (`self.MonsterTurnLeft`)
        (goto _label_3)
        (else
          (goto _label_5))))))

(event `MonsterTurnUp`
  (`self.CheckActionDirection` "Up")
  (`self.Set Action Direction` (`self.Direction`) :!label _label_6))

(event `MonsterTurnDown`
  (`self.CheckActionDirection` "Down")
  (goto _label_6))

(event `MonsterTurnLeft`
  (`self.CheckActionDirection` "Left")
  (goto _label_6))

(event `BlockedByPlayer`
  ;[0 0 0] BlockedByPlayer/WallThen
  (set `self.WillPlayerMove?` false :!label _label_7))

(event `BlockedByWall`
  ;[0 0 0] BlockedByPlayer/WallThen
  (goto _label_7))

(event `MonsterTurnRight`
  (`self.CheckActionDirection` "Right")
  (goto _label_6))

(event `MonsterMove`
  (bind (_direction _120bpm) (`Timeline|时间轴` :!via `PlayFromStart`)
    (:`Update`
      (`self.K2_SetActorLocation` (`KismetMathLibrary.VLerp` (`self.MonsterLocation`) (`self.NextLocation`) _120bpm))
      (set `self.WillPlayerMove?` false))))

(event `MonsterCharge`
  (`SceneComponent.SetVisibility` (`self.AoeVisual`) true false)
  (set `self.WillPlayerMove?` false :!label _label_8))

(event `MonsterAttack`
  ;[1 1 1] 注释
  (`self.MonsterCharge`)
  (`KismetSystemLibrary.Delay` 0.5)
  (`KismetSystemLibrary.DelayUntilNextTick`)
  (`self.MonsterSkill` 0)
  (goto _label_8))

(event `MonsterSkill`
  (params (Sort :type Integer))
  (`/Engine/EditorBlueprintResources/StandardMacros.IsValid` self
    (:`Is Valid`
      (bind _willhitplayer_ (`self.CheckSkillHit`))
      (if _willhitplayer_
        (bind _asbp_my_game_mode (cast `/Game/Character/BP_MyGameMode` (`GameplayStatics.GetGameMode`)))
        (`/Game/Character/BP_MyGameMode.AlterThePlayerHP` _asbp_my_game_mode "Skill" 1)
        (`KismetSystemLibrary.DelayUntilNextTick`)
        (set `self.WillPlayerMove?` false)
        ;[1 1 1] 注释
        (`KismetSystemLibrary.PrintString` "被打了！！" true true (struct :`R` 1.0 :`G` 0.011477 :`A` 1.0) 20.0)))))

(event `MonsterSkillVisual`
  (bind _aoevfx (`self.AoeVFX`))
  (`SceneComponent.SetVisibility` (`self.AoeVisual`) false false)
  (`SceneComponent.SetVisibility` _aoevfx true false)
  (`PaperFlipbookComponent.PlayFromStart` _aoevfx)
  (`KismetSystemLibrary.Delay` (`PaperFlipbookComponent.GetFlipbookLength` (`self.AoeVFX`)))
  (`SceneComponent.SetVisibility` (`self.AoeVFX`) false false))

(event `MonsterDie`
  ;[1 1 1] 注释
  (`KismetSystemLibrary.PrintString` "BOSS HP-1")
  (`GameplayStatics.PlaySound2D` "/Game/SFX/FFXIV/FFXIV_Remove_Item.FFXIV_Remove_Item" 1.0 1.0 0.0 null null)
  (set `self.WillPlayerMove?` false)
  (`self.K2_DestroyActor`))

(fn `Check Blocked by Player or Wall`
  (returns (BlockedType :type String))
  ;[0 0 0] BlockedByPlayer?
  (if (`KismetStringLibrary.IsEmpty` (`/Game/Character/BP_Player.Direction` (`self.ThePlayer`)))
    (if (`PrimitiveComponent.IsOverlappingComponent` (`self.NextStep`) (`Character.CapsuleComponent` (`self.ThePlayer`)))
      _
      (else
        ;[0 0 0] BlockedByWall?
        (if (`KismetArrayLibrary.Array_IsNotEmpty` (`PrimitiveComponent.GetOverlappingActors` (`self.NextStep`) "/Game/Actor/BP_Wall.BP_Wall_C")) :!label _label
          (return "Wall")
          (else
            (return "Nothing")))))
    (elif (`PrimitiveComponent.IsOverlappingComponent` (`self.NextStep`) (`/Game/Character/BP_Player.NextStep` (`self.ThePlayer`)))
      _
      (else
        (goto _label))))
  (return "Player"))

(fn `CheckActionDirection`
  (params (Direction :type String))
  (set `self.MonsterLocation` (`self.K2_GetActorLocation`))
  (set `self.Direction` Direction))

(fn `CheckSkillHit`
  (returns (`WillHitPlayer?` :type Boolean))
  (if (`self.WillPlayerMove?`)
    (if (`PrimitiveComponent.IsOverlappingComponent` (`self.AoeCollision`) (`/Game/Character/BP_Player.NextStep` (`self.ThePlayer`)))
      (return true)
      (else
        _))
    (elif (`PrimitiveComponent.IsOverlappingComponent` (`self.AoeCollision`) (`Character.CapsuleComponent` (`self.ThePlayer`)))
      (return true)
      (else
        _)))
  (return false))

(fn `Set Action Direction`
  (params (Direction :type String))
  (switch `string` Direction
    (:`Up`
      (`SceneComponent.K2_SetRelativeLocation` (`self.NextStep`) (200.0 0.0 0.0) false false)
      (`SceneComponent.K2_SetRelativeLocation` (`self.AoeCollision`) (200.0 0.0 0.0) false false))
    (:`Down`
      (`SceneComponent.K2_SetRelativeLocation` (`self.NextStep`) (-200.0 0.0 0.0) false false)
      (`SceneComponent.K2_SetRelativeLocation` (`self.AoeCollision`) (-200.0 0.0 0.0) false false))
    (:`Right`
      (`SceneComponent.K2_SetRelativeLocation` (`self.NextStep`) (0.0 200.0 0.0) false false)
      (`SceneComponent.K2_SetRelativeLocation` (`self.AoeCollision`) (0.0 200.0 0.0) false false)
      (`SceneComponent.K2_SetRelativeRotation` (`self.PaperFlipbook`) (struct :`Pitch` 180.0 :`Yaw` 90.0 :`Roll` -90.0) false false))
    (:`Left`
      (`SceneComponent.K2_SetRelativeLocation` (`self.NextStep`) (0.0 -200.0 0.0) false false)
      (`SceneComponent.K2_SetRelativeLocation` (`self.AoeCollision`) (0.0 -200.0 0.0) false false)
      (`SceneComponent.K2_SetRelativeRotation` (`self.PaperFlipbook`) (struct :`Yaw` 90.0 :`Roll` -90.0) false false)))
  (set `self.NextLocation` (`SceneComponent.K2_GetComponentLocation` (`self.NextStep`)))
  (return))

(fn `SetBeat`
  (if (== (`self.Beat`) 3)
    (set `self.Beat` 0)
    (else
      (`/Engine/EditorBlueprintResources/StandardMacros.IncrementInt` (`self.Beat`)
        (:`  `
          _))))
  (return))

(fn `UserConstructionScript`)