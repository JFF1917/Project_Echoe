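; BP_Monster_Item_Recover is a monster-style item actor that, judging by its name, serves as a recovery pickup.
; On MonsterDie it calls AlterThePlayerHP on BP_MyGameMode with a skill type, a value of negative one and a sound cue.
; It then clears WillPlayerMove and destroys itself; the remaining events and construction script add no logic of their own.
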(event `self.MonsterDie`
  (bind _asbp_my_game_mode (cast `/Game/Character/BP_MyGameMode` (`GameplayStatics.GetGameMode`)))
  (`/Game/Character/BP_MyGameMode.AlterThePlayerHP` _asbp_my_game_mode "Skill" -1 "/Game/SFX/FFXIV/FFXIV_Cancel.FFXIV_Cancel")
  (set `self.WillPlayerMove?` false)
  (`self.K2_DestroyActor`))

(fn `UserConstructionScript`
  (`parent.UserConstructionScript`))