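; Bat monster Blueprint that defines patrol and chase-and-attack behaviour as overrides of numbered action events.
; Patrol actions P2 and P4 check for blockers, hand off to player or wall handlers, or turn left and right respectively before moving.
; Chase actions CA2 and CA4 both chase the player, and being blocked by the player triggers an attack.
; The parent BeginPlay call is a disabled placeholder node.
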(event `self.ActionP2`
  ;[0 0 0] BatPatrol
  (bind _blockedtype (`self.Check Blocked by Player or Wall`))
  (switch `string` _blockedtype
    (:`Player`
      (`self.BlockedByPlayer`))
    (:`Wall`
      (`self.BlockedByWall`))
    (:`Nothing`
      (`self.MonsterTurnLeft`)
      (`self.MonsterMove` :!label _label))))

(event `self.ActionP4`
  ;[0 0 0] BatPatrol
  (bind _blockedtype (`self.Check Blocked by Player or Wall`))
  (switch `string` _blockedtype
    (:`Player`
      (`self.BlockedByPlayer`))
    (:`Wall`
      (`self.BlockedByWall`))
    (:`Nothing`
      (`self.MonsterTurnRight`)
      (goto _label))))

(event `self.ActionCA2`
  ;[0 0 0] BatChase&Attack
  (`self.MonsterChasePlayer` :!label _label_2))

(event `self.BlockedByPlayer`
  (`self.MonsterAttack`))

(event `self.ActionCA4`
  ;[0 0 0] BatChase&Attack
  (goto _label_2))

(fn `UserConstructionScript`
  (`parent.UserConstructionScript`))