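; BP_Monster_Sword is a monster actor whose construction script picks one of four seed flipbooks by Sort for cores, and clears the flipbook otherwise.
; ShowShield, HideShield and DestroyShield are empty stubs, and BeginPlay's parent call is disabled.
; Disconnected graph logic would hide the current shield, or size an AoE beam: fixed by orientation for cores, otherwise stretched by distance to a random connected shield.
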(event `ShowShield`
  ;[1 1 1] 注释
)

(event `HideShield`
  ;[1 1 1] 注释
)

(event `DestroyShield`
  ;[1 1 1] 注释
)

(fn `UserConstructionScript`
  (`parent.UserConstructionScript`)
  ;[0 0 0] 初始化
  (if (`self.IsCore?`)
    (switch `int` (`self.Sort`)
      (:`1`
        (`PaperFlipbookComponent.SetFlipbook` (`self.PaperFlipbook`) "/Game/Actor/Anim/Anim_Seed_1.Anim_Seed_1"))
      (:`2`
        (`PaperFlipbookComponent.SetFlipbook` (`self.PaperFlipbook`) "/Game/Actor/Anim/Anim_Seed_2.Anim_Seed_2"))
      (:`3`
        (`PaperFlipbookComponent.SetFlipbook` (`self.PaperFlipbook`) "/Game/Actor/Anim/Anim_Seed_3.Anim_Seed_3"))
      (:`4`
        (`PaperFlipbookComponent.SetFlipbook` (`self.PaperFlipbook`) "/Game/Actor/Anim/Anim_Seed_4.Anim_Seed_4")))
    (else
      (`PaperFlipbookComponent.SetFlipbook` (`self.PaperFlipbook`) null))))