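; BP_MyGameMode is the game mode for a beat-driven game, handling menu setup, game start and HP changes.
; BeginPlay caches player and game instance, then creates the save object and widgets.
; GameStart restores HP and controls, then loops music with a 120 BPM timeline that cues the game view's bars.
; PlayABeat triggers the player's action, then every monster's a tick later; damage events call death at zero HP.
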(event `self.ReceiveBeginPlay`
  (bind _asbp_my_game_instance (cast `/Game/Character/BP_MyGameInstance` (`GameplayStatics.GetGameInstance`)))
  (set `self.My Game Instance` _asbp_my_game_instance)
  (bind _asbp_player (cast `/Game/Character/BP_Player` (`GameplayStatics.GetPlayerCharacter` 0)))
  (set `self.ThePlayer` _asbp_player)
  (bind _returnvalue (`GameplayStatics.CreateSaveGameObject` "/Game/Character/BP_MySaveGame.BP_MySaveGame_C"))
  (set `/Game/Character/BP_MyGameInstance.MySaveGame_Ins` _returnvalue (`self.My Game Instance`))
  (`|ExecutionSequence`
    (:`then_0`
      ;[0 0 0] CreateWidget
      (bind _returnvalue_2 (`|CreateWidget` "/Game/Widget/WBP_MainMenu.WBP_MainMenu_C"))
      (bind _output_get (set `/Game/Character/BP_MyGameInstance.WBP_MainMenu_Ins` _returnvalue_2 (`self.My Game Instance`)))
      (`self.Add Widget to Viewport PC` _output_get)
      (bind _returnvalue_3 (`|CreateWidget` "/Game/Widget/WBP_GameView.WBP_GameView_C"))
      (set `/Game/Character/BP_MyGameInstance.WBP_GameView_Ins` _returnvalue_3 (`self.My Game Instance`)))))

(event `GameStart`
  (`|ExecutionSequence`
    (:`then_0`
      (`/Game/Character/BP_Player.ResetPlayerHP` (`self.ThePlayer`))
      (`/Game/Character/BP_Player.Add PlayerControlAsUnit IMC` (`self.ThePlayer`))
      (set `PlayerController.bShowMouseCursor` false (`GameplayStatics.GetPlayerController` 0)))
    (:`then_1`
      (`UserWidget.AddToViewport` (`/Game/Character/BP_MyGameInstance.WBP_GameView_Ins` (`self.My Game Instance`)) 0)
      (`self.PlayABeat`))
    (:`then_2`
      (`GameplayStatics.PlaySound2D` "/Game/SFX/BGM/BGM_FreeCity_S1.BGM_FreeCity_S1" 1.0 1.0 0.0 null null)
      (`|ExecutionSequence`
        (:`then_0`
          (`KismetSystemLibrary.Delay` 2.3)
          (`|ExecutionSequence` :!label _label
            (:`then_0`
              (`GameplayStatics.PlaySound2D` "/Game/SFX/BGM/BGM_FreeCity_S2.BGM_FreeCity_S2" 1.0 1.0 0.0 null null))
            (:`then_1`
              (`Timeline|BGM120BPM` :!via `PlayFromStart`
                (:`Finished`
                  (goto _label))
                (:`S2`
                  (`KismetSystemLibrary.Delay` 0.1)
                  (`/Game/Widget/WBP_GameView.PlayABar` (`/Game/Character/BP_MyGameInstance.WBP_GameView_Ins` (`self.My Game Instance`))))))))
        (:`then_1`
          (`PaperFlipbookComponent.SetFlipbook` (`/Game/Actor/BP_FloorBeat.PaperFlipbook` (`/Game/Character/BP_Player.FloorBeat` (`self.ThePlayer`))) "/Game/Actor/Texture/Anim_FloorBeat.Anim_FloorBeat"))))))

(event `AlterPlayerHP`
  (params (Type :type Name) (AlterHPValue :type Integer))
  (bind _theplayer (`self.ThePlayer`))
  (switch `name` Type
    (:`Skill`
      (bind _output_get (set `/Game/Character/BP_Player.PlayerHP` (- (`/Game/Character/BP_Player.PlayerHP` _theplayer) AlterHPValue) _theplayer))
      (if (< _output_get 1)
        (`/Game/Character/BP_Player.PlayerDie` _theplayer)))))

(event `AlterMonsterHP`
  (params (Damage :type Integer) (TheMonster :type "/Game/Actor/BP_MonsterBase Object Reference"))
  (bind _output_get (set `/Game/Actor/BP_MonsterBase.MonsterHP` (- (`/Game/Actor/BP_MonsterBase.MonsterHP` TheMonster) Damage) TheMonster))
  (if (< _output_get 1)
    (`/Game/Actor/BP_MonsterBase.MonsterDie` TheMonster)))

(event `PlayABeat`
  ;[0 0 0] 注释
  (`/Game/Character/BP_Player.Action` (`self.ThePlayer`))
  (`KismetSystemLibrary.DelayUntilNextTick`)
  ;[0 0 0] 注释
  (bind _outactors (`GameplayStatics.GetAllActorsOfClass` "/Game/Actor/BP_MonsterBase.BP_MonsterBase_C"))
  (for _array_element _outactors
    (`/Engine/EditorBlueprintResources/StandardMacros.IsValid` _array_element
      (:`Is Valid`
        (`/Game/Actor/BP_MonsterBase.MonsterAction` _array_element)))))

(event `PlayABar`
  ;[1 1 1] 注释
  (`Timeline|BPM` :!via `PlayFromStart`
    (:`Light`
      ;[1 1 1] 注释
      (`KismetSystemLibrary.PrintString` "————————" true true (struct :`G` 1.0 :`B` 0.030675 :`A` 1.0) 5.0))
    (:`Heavy`
      (`KismetSystemLibrary.PrintString` "——————————————" true true (struct :`R` 1.0 :`B` 0.073803 :`A` 1.0) 5.0))))

(fn `Add Widget to Viewport PC`
  (params (`WBP Ins` :type "UserWidget Object Reference"))
  (`UserWidget.AddToViewport` `WBP Ins` 0)
  (set `PlayerController.bShowMouseCursor` true (`GameplayStatics.GetPlayerController` 0)))

(fn `Create Ins Array`
  (params (LastIndex :type Integer) (TargetArray :type "Array of Actor Object Reference (by ref)") (Class :type "Actor Class Reference") (`Spawn Transform Location` :type "Vector Structure"))
  (for _ (range (+ LastIndex 1))
    (bind _returnvalue (`|SpawnActorFromClass` Class (`KismetMathLibrary.MakeTransform` `Spawn Transform Location`) "Undefined" "MultiplyWithRoot" null null))
    (`KismetArrayLibrary.Array_Add` TargetArray _returnvalue)))

(fn `UserConstructionScript`)