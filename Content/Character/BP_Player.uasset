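; Player pawn for a 2D flipbook game, switching between free movement and grid-step "unit" control through Enhanced Input mapping contexts.
; Directional inputs aim the weapon and next-step probe; Action then attacks overlapping monsters through the game mode, or timeline-lerps a step unless a wall blocks it.
; Action also flags all monsters that the player will move.
; It also handles hit/heal flashes, start-room locking with BGM change, and death into the game-over screen.
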(event `Lock`
  (params (OverlappedActor :type "Actor Object Reference") (OtherActor :type "Actor Object Reference"))
  ;[0 0 0] LockStartRoom
  (`SceneComponent.SetVisibility` (`/Game/Actor/BP_Lock.Sprite_Floor_Lock` (`self.LockSprite`)) true true)
  (`PrimitiveComponent.SetCollisionEnabled` (`/Game/Actor/BP_Wall.Box` (`self.LockWall`)) "QueryOnly")
  (`self.K2_DestroyActor` (`self.LockTriggerBox`))
  (`/Game/Character/BP_MyGameMode.BGMChange` (`self.MyGameMode`)))

(event `self.ReceiveBeginPlay`
  (set `/Game/Widget/BP_PaperFlipBook.ThePlayer` self (`self.UICorePaperFilpBook`))
  (bind _asbp_my_game_mode (cast `/Game/Character/BP_MyGameMode` (`GameplayStatics.GetGameMode`)))
  (set `self.MyGameMode` _asbp_my_game_mode)
  (bind _asbp_my_game_instance (cast `/Game/Character/BP_MyGameInstance` (`GameplayStatics.GetGameInstance`)))
  (set `self.MyGameInstance` _asbp_my_game_instance)
  ;[0 0 0] LockStartRoom
  (add `self.OnActorBeginOverlap` (`self.LockTriggerBox`) (delegate `Lock`)))

(event `Action`
  (if (not (`KismetStringLibrary.IsEmpty` (`self.Direction`)))
    (bind _outactors (`GameplayStatics.GetAllActorsOfClass` "/Game/Actor/BP_MonsterBase.BP_MonsterBase_C"))
    (for _array_element _outactors
      (set `/Game/Actor/BP_MonsterBase.WillPlayerMove?` true _array_element))
    (for _array_element_2 _outactors
      (if (`PrimitiveComponent.IsOverlappingComponent` (`self.AttackBox`) (`/Game/Actor/BP_MonsterBase.SelfCollission` _array_element_2))
        (set `self.CanAttack?` true)
        (break)))
    (if (`self.CanAttack?`)
      (`self.Attack`)
      (set `self.CanAttack?` false)
      (elif (not (`KismetArrayLibrary.Array_IsNotEmpty` (`PrimitiveComponent.GetOverlappingActors` (`self.NextStep`) "/Game/Actor/BP_Wall.BP_Wall_C")))
        (`self.Move`)))
    (set `self.Direction` "")))

(event `Attack`
  (`|ExecutionSequence`
    (:`then_0`
      (`SceneComponent.SetVisibility` (`self.AoeVFX`) true false)
      (`PaperFlipbookComponent.PlayFromStart` (`self.AoeVFX`))
      (`KismetSystemLibrary.Delay` (`PaperFlipbookComponent.GetFlipbookLength` (`self.AoeVFX`)))
      (`SceneComponent.SetVisibility` (`self.AoeVFX`) false false))
    (:`then_1`
      (bind _outactors (`GameplayStatics.GetAllActorsOfClass` "/Game/Actor/BP_MonsterBase.BP_MonsterBase_C"))
      (for _array_element _outactors
        (bind _output_get (set `self.TheMonster` _array_element))
        (if (`PrimitiveComponent.IsOverlappingComponent` (`self.AttackBox`) (`/Game/Actor/BP_MonsterBase.SelfCollission` _output_get))
          (`/Game/Character/BP_MyGameMode.AlterMonsterHP` (`self.MyGameMode`) (`self.SkillDamage`) (`self.TheMonster`)))))))

(event `PlayerDie`
  (bind _wbp_gameover_ins (`/Game/Character/BP_MyGameInstance.WBP_GameOver_Ins` (`self.MyGameInstance`)))
  (bind _currentbgm (`/Game/Character/BP_MyGameMode.CurrentBGM` (`self.MyGameMode`)))
  (`self.Delete PlayerControlAsUnit IMC`)
  (`Widget.RemoveFromParent` (`/Game/Character/BP_MyGameInstance.WBP_GameView_Ins` (`self.MyGameInstance`)))
  (`/Game/Widget/WBP_GameOver.SetLook` _wbp_gameover_ins false)
  (`self.AddWidgetToViewportPC` _wbp_gameover_ins)
  ;[0 0 0] CutMusic
  (`AudioComponent.FadeOut` _currentbgm 1.0 0.0 "Linear")
  (`AudioComponent.SetSound` _currentbgm null)
  (`GameplayStatics.PlaySound2D` "/Game/SFX/FFXIV/FFXIV_Instance_Failed.FFXIV_Instance_Failed" 1.0 1.0 0.0 null null))

(event `PlayerDamageVFX`
  (`PaperFlipbookComponent.SetSpriteColor` (`self.Sprite`) (struct :`R` 1.0 :`A` 1.0))
  (`KismetSystemLibrary.Delay` 0.1)
  (`PaperFlipbookComponent.SetSpriteColor` (`self.Sprite`) (struct :`R` 1.0 :`G` 1.0 :`B` 1.0 :`A` 1.0))
  (`KismetSystemLibrary.Delay` 0.05)
  (`PaperFlipbookComponent.SetSpriteColor` (`self.Sprite`) (struct :`R` 1.0 :`A` 1.0))
  (`KismetSystemLibrary.Delay` 0.1)
  (`PaperFlipbookComponent.SetSpriteColor` (`self.Sprite`) (struct :`R` 1.0 :`G` 1.0 :`B` 1.0 :`A` 1.0))
  (`KismetSystemLibrary.Delay` 0.05)
  (`PaperFlipbookComponent.SetSpriteColor` (`self.Sprite`) (struct :`R` 1.0 :`A` 1.0))
  (`KismetSystemLibrary.Delay` 0.1)
  (`PaperFlipbookComponent.SetSpriteColor` (`self.Sprite`) (struct :`R` 1.0 :`G` 1.0 :`B` 1.0 :`A` 1.0)))

(event `PlayerCureVFX`
  (`PaperFlipbookComponent.SetSpriteColor` (`self.Sprite`) (struct :`R` 1.0 :`G` 1.0 :`A` 1.0))
  (`KismetSystemLibrary.Delay` 0.1)
  (`PaperFlipbookComponent.SetSpriteColor` (`self.Sprite`) (struct :`R` 1.0 :`G` 1.0 :`B` 1.0 :`A` 1.0))
  (`KismetSystemLibrary.Delay` 0.05)
  (`PaperFlipbookComponent.SetSpriteColor` (`self.Sprite`) (struct :`R` 0.835104 :`G` 1.0 :`A` 1.0))
  (`KismetSystemLibrary.Delay` 0.1)
  (`PaperFlipbookComponent.SetSpriteColor` (`self.Sprite`) (struct :`R` 1.0 :`G` 1.0 :`B` 1.0 :`A` 1.0))
  (`KismetSystemLibrary.Delay` 0.05)
  (`PaperFlipbookComponent.SetSpriteColor` (`self.Sprite`) (struct :`R` 1.0 :`G` 1.0 :`A` 1.0))
  (`KismetSystemLibrary.Delay` 0.1)
  (`PaperFlipbookComponent.SetSpriteColor` (`self.Sprite`) (struct :`R` 1.0 :`G` 1.0 :`B` 1.0 :`A` 1.0)))

(event `EnhancedInput|/Game/Input/IA_Up`
  (params (ActionValue :type Boolean) (ElapsedSeconds :type "Float (double-precision)") (TriggeredSeconds :type "Float (double-precision)") (InputAction :type "InputAction Object Reference" :default "/Game/Input/IA_Up.IA_Up"))
  ;[0 0 0] UnitPlayerMove
  (:`Triggered`
    (`self.CheckActionDirection` "Up")
    (`self.SetActionDirection` (`self.Direction`) :!label _label)))

(event `EnhancedInput|/Game/Input/IA_Move`
  (params (ActionValue :type "Vector2D Structure") (ElapsedSeconds :type "Float (double-precision)") (TriggeredSeconds :type "Float (double-precision)") (InputAction :type "InputAction Object Reference" :default "/Game/Input/IA_Move.IA_Move"))
  (bind (_returnvalue_roll _returnvalue_pitch _returnvalue_yaw) (`KismetMathLibrary.BreakRotator` (`self.GetControlRotation`)))
  (bind (_returnvalue_roll_2 _returnvalue_pitch_2 _returnvalue_yaw_2) (`KismetMathLibrary.BreakRotator` (`self.GetControlRotation`)))
  ;[0 0 0] FreePlayerMove
  (:`Triggered`
    (`self.AddMovementInput` (`KismetMathLibrary.GetRightVector` (`KismetMathLibrary.MakeRotator` _returnvalue_roll_2 0.0 _returnvalue_yaw_2)) ActionValue_X)
    (`self.AddMovementInput` (`KismetMathLibrary.GetForwardVector` (`KismetMathLibrary.MakeRotator` 0.0 0.0 _returnvalue_yaw)) ActionValue_Y))
  (:`Started`
    (`PaperFlipbookComponent.SetFlipbook` (`self.Sprite`) "/Game/Character/TestAnim/2DAni_Chara_Run.2DAni_Chara_Run"))
  (:`Completed`
    (`PaperFlipbookComponent.SetFlipbook` (`self.Sprite`) "/Game/Character/TestAnim/2DAni_Chara_Wait.2DAni_Chara_Wait")))

(event `EnhancedInput|/Game/Input/IA_Down`
  (params (ActionValue :type Boolean) (ElapsedSeconds :type "Float (double-precision)") (TriggeredSeconds :type "Float (double-precision)") (InputAction :type "InputAction Object Reference" :default "/Game/Input/IA_Down.IA_Down"))
  ;[0 0 0] UnitPlayerMove
  (:`Triggered`
    (`self.CheckActionDirection` "Down")
    (goto _label)))

(event `EnhancedInput|/Game/Input/IA_Left`
  (params (ActionValue :type Boolean) (ElapsedSeconds :type "Float (double-precision)") (TriggeredSeconds :type "Float (double-precision)") (InputAction :type "InputAction Object Reference" :default "/Game/Input/IA_Left.IA_Left"))
  ;[0 0 0] UnitPlayerMove
  (:`Triggered`
    (`self.CheckActionDirection` "Left")
    (goto _label)))

(event `EnhancedInput|/Game/Input/IA_Right`
  (params (ActionValue :type Boolean) (ElapsedSeconds :type "Float (double-precision)") (TriggeredSeconds :type "Float (double-precision)") (InputAction :type "InputAction Object Reference" :default "/Game/Input/IA_Right.IA_Right"))
  ;[0 0 0] UnitPlayerMove
  (:`Triggered`
    (`self.CheckActionDirection` "Right")
    (goto _label)))

(event `Key|A`
  (params (Key :type "Key Structure"))
  ;[0 0 0] FreePlayerMove
)

(event `Key|D`
  (params (Key :type "Key Structure"))
  ;[0 0 0] FreePlayerMove
)

(event `Move`
  ;[0 0 0] UnitPlayerMove
  (bind (_direction _120bpm) (`Timeline|时间轴` :!via `PlayFromStart`)
    (:`Update`
      (`self.K2_SetActorLocation` (`KismetMathLibrary.VLerp` (`self.PlayerLocation`) (`self.NextLocation`) _120bpm)))))

(event `Add PlayerControl IMC`
  ;[0 0 0] FreePlayerMove
  (bind `_as玩家控制器` (cast `PlayerController` (`self.GetController`)))
  (bind _returnvalue (pcsubsystem `EnhancedInputLocalPlayerSubsystem` `_as玩家控制器`))
  (`/Engine/EditorBlueprintResources/StandardMacros.IsValid` _returnvalue
    (:`Is Valid`
      (`EnhancedInputSubsystemInterface.AddMappingContext` _returnvalue "/Game/Input/IMC_PlayerControl.IMC_PlayerControl" 0 (struct)))))

(event `Add PlayerControlAsUnit IMC`
  (bind `_as玩家控制器` (cast `PlayerController` (`self.GetController`)))
  (bind _returnvalue (pcsubsystem `EnhancedInputLocalPlayerSubsystem` `_as玩家控制器`))
  (`/Engine/EditorBlueprintResources/StandardMacros.IsValid` _returnvalue
    (:`Is Valid`
      (`EnhancedInputSubsystemInterface.AddMappingContext` _returnvalue "/Game/Input/IMC_PlayerControlAsUnit.IMC_PlayerControlAsUnit" 0 (struct)))))

(event `Delete PlayerControl IMC`
  ;[0 0 0] FreePlayerMove
  (bind `_as玩家控制器` (cast `PlayerController` (`self.GetController`)))
  (bind _returnvalue (pcsubsystem `EnhancedInputLocalPlayerSubsystem` `_as玩家控制器`))
  (`/Engine/EditorBlueprintResources/StandardMacros.IsValid` _returnvalue
    (:`Is Valid`
      (`EnhancedInputSubsystemInterface.RemoveMappingContext` _returnvalue "/Game/Input/IMC_PlayerControl.IMC_PlayerControl" (struct)))))

(event `Delete PlayerControlAsUnit IMC`
  (bind `_as玩家控制器` (cast `PlayerController` (`self.GetController`)))
  (bind _returnvalue (pcsubsystem `EnhancedInputLocalPlayerSubsystem` `_as玩家控制器`))
  (`/Engine/EditorBlueprintResources/StandardMacros.IsValid` _returnvalue
    (:`Is Valid`
      (`EnhancedInputSubsystemInterface.RemoveMappingContext` _returnvalue "/Game/Input/IMC_PlayerControlAsUnit.IMC_PlayerControlAsUnit" (struct)))))

(fn `AddWidgetToViewportPC`
  (params (WBP_Ins :type "UserWidget Object Reference"))
  (`UserWidget.AddToViewport` WBP_Ins 0)
  (set `PlayerController.bShowMouseCursor` true (`GameplayStatics.GetPlayerController` 0)))

(fn `CheckActionDirection`
  (params (Direction :type String))
  (if (`self.CanAction?`)
    (set `self.PlayerLocation` (`self.K2_GetActorLocation`))
    (set `self.Direction` Direction)))

(fn `ResetPlayerHP`
  (set `self.PlayerHP` (`self.PlayerHPMax`)))

(fn `SetActionDirection`
  (params (Direction :type String))
  (switch `string` Direction
    (:`Up`
      (`SceneComponent.K2_SetRelativeLocation` (`self.WeaponLocation`) (0.0 0.0 200.0) false false)
      (`SceneComponent.K2_SetRelativeLocation` (`self.NextStep`) (0.0 0.0 200.0) false false))
    (:`Down`
      (`SceneComponent.K2_SetRelativeLocation` (`self.WeaponLocation`) (0.0 0.0 -200.0) false false)
      (`SceneComponent.K2_SetRelativeLocation` (`self.NextStep`) (0.0 0.0 -200.0) false false))
    (:`Right`
      (`SceneComponent.K2_SetRelativeLocation` (`self.WeaponLocation`) (0.0 200.0 0.0) false false)
      (`SceneComponent.K2_SetRelativeLocation` (`self.NextStep`) (0.0 200.0 0.0) false false)
      (`SceneComponent.K2_SetRelativeRotation` (`self.Sprite`) (struct :`Yaw` -90.0) false false))
    (:`Left`
      (`SceneComponent.K2_SetRelativeLocation` (`self.WeaponLocation`) (0.0 -200.0 0.0) false false)
      (`SceneComponent.K2_SetRelativeLocation` (`self.NextStep`) (0.0 -200.0 0.0) false false)
      (`SceneComponent.K2_SetRelativeRotation` (`self.Sprite`) (struct :`Yaw` 90.0) false false)))
  (set `self.NextLocation` (`SceneComponent.K2_GetComponentLocation` (`self.NextStep`)))
  (return))

(fn `UserConstructionScript`)